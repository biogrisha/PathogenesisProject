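; Enemy turret that detects the Player-tagged character by facing angle and line of sight, or when damaged by it, then tracks and shoots it.
; Bound tick events run detection and constant-speed top rotation, while a looping timer, paused when not aiming, spawns projectiles once tightly aligned.
; A health component drives the widget bar and death.
; A save proxy registered with the game mode restores location and health, saving on death or quit.
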(event Custom|StartAiming
  (EventDispatchers|BindEventtoTickEvents (delegate Custom|AimEvent))
  (Utilities|Time|UnpauseTimerbyHandle (Variables|Default|GetShootingTimer)))

(event Custom|Aim
  (params (DeltaTime :type Float%20%28single-precision%29))
  (bind _aimactor (Variables|Default|GetAimActor))
  (bind _returnvalue (Transformation|GetActorLocation _aimactor))
  (Utilities|IsValid _aimactor
    (:Is%20Valid
      (if (Math|Vector|NotEqual(Vector) _returnvalue (Variables|Default|GetAimLocationTemp) 0.0001)
        (bind _output_get (Variables|Default|SetAimRotation (Math|Rotator|FindLookatRotation (Transformation|GetWorldLocation (Variables|Default|GetStaticMeshTop)) _returnvalue))))
      (Variables|Default|SetAimLocationTemp _returnvalue)
      (Transformation|SetWorldRotation (Variables|Default|GetStaticMeshTop) (Class|KismetMathLibrary|RInterptoConstant (Transformation|GetWorldRotation (Variables|Default|GetStaticMeshTop)) _output_get DeltaTime (Variables|Default|GetAimSpeed)) false false))))

(event Custom|DeathEvent
  ;[1 1 1] Death
  (CallFunction|Save)
  (Actor|DestroyActor))

(event Custom|AimEvent
  (params (DeltaTime :type Float%20%28single-precision%29))
  (CallFunction|Aim DeltaTime))

(event Custom|Behaviour
  (bind _aimactor (Variables|Default|GetAimActor))
  (Utilities|IsValid _aimactor
    (:Is%20Valid
      (if (Variables|Default|GetIsAiming)
        ;[1 1 1] Stop aiming if lose sight
        (bind _result (CallFunction|HasLineOfSight _aimactor))
        (if (not _result)
          (CallFunction|StopAiming)
          (Variables|Default|SetIsAiming false))
        (else
          ;[1 1 1] Start aiming player if detected
          (bind _result_2 (CallFunction|IsAimed (Transformation|GetActorLocation _aimactor) 0.7))
          (bind _result_3 (CallFunction|HasLineOfSight _aimactor))
          (if (and _result_3 _result_2)
            (CallFunction|StartAiming)
            (Variables|Default|SetIsAiming true)))))))

(event Custom|Save
  (bind _output_get (Variables|Default|SetSaveData (Utilities|Struct|MakeDataToSave (Transformation|GetActorLocation) (Class|GHealthComponent|GetHealth (Variables|Default|GetTurretHealth)) true)))
  (Class|GSaveDataProxy|SetData (Variables|Default|GetSaveDataProxy) _output_get))

(event Custom|Shoot
  (bind _aimactor (Variables|Default|GetAimActor))
  (bind _barrelendl (Variables|Default|GetBarrelEndL))
  (bind _returnvalue (Transformation|GetWorldTransform _barrelendl))
  (Utilities|IsValid _aimactor
    (:Is%20Valid
      (bind _result (CallFunction|IsAimed (Transformation|GetActorLocation _aimactor) 0.99))
      (if _result
        (bind _returnvalue_2 (Game|SpawnActorfromClass "/Game/MyContent/Blueprints/Weapons/Projectile.Projectile_C" (Math|Transform|MakeTransform (.location _returnvalue) (.rotation _returnvalue) "1,1,1") "AdjustIfPossibleButAlwaysSpawn" 0 0))
        (Variables|/Game/MyContent/Blueprints/Weapons/Projectile.Projectile_C|SetDamage _returnvalue_2 (Variables|Default|GetDamage))
        (Variables|/Game/MyContent/Blueprints/Weapons/Projectile.Projectile_C|SetShooter _returnvalue_2 self)))))

(event Custom|CreateSaveDataProxy
  (bind _returnvalue (Game|GetGameMode))
  (bind _returnvalue_2 (Game|ConstructObjectfromClass "/Script/PathogenesisProject.GSaveDataProxy" _returnvalue))
  (bind _output_get (Variables|Default|SetSaveDataProxy _returnvalue_2))
  (Class|GSaveDataProxy|SetData _output_get (Utilities|Struct|MakeDataToSave (Transformation|GetActorLocation) (Class|GHealthComponent|GetHealth (Variables|Default|GetTurretHealth)) false))
  (Class|GSaveDataProxy|SetStoredObjectName _output_get (Utilities|GetObjectName self))
  (bind _asbp_start_game_mode (Utilities|Casting|CastToBP_StartGameMode _returnvalue))
  (Default|SubscribeSaveDataProxy _asbp_start_game_mode _output_get)
  (bind _returnvalue_3 (Class|GSaveDataProxy|GetData _output_get))
  (Variables|Default|SetSaveData _returnvalue_3))

(event Custom|InitFromSave
  (bind _savedata (Variables|Default|GetSaveData))
  (Transformation|SetActorLocation (.location _savedata) false false)
  (Class|GHealthComponent|SetHealth (Variables|Default|GetTurretHealth) (.health _savedata)))

(event Custom|ShootingEvent
  ;[1 1 1] prepare shooting timer
  (CallFunction|Shoot))

(event Custom|SaveEvent
  ;[1 1 1] Init From Save Data
  (CallFunction|Save))

(event Custom|StopAiming
  (EventDispatchers|UnbindEventfromTickEvents (delegate Custom|AimEvent))
  (Utilities|Time|PauseTimerbyHandle (Variables|Default|GetShootingTimer)))

(event Custom|BehaviourEvent
  (params (DeltaTime :type Float%20%28single-precision%29))
  ;[1 1 1] Start behaviour
  (CallFunction|Behaviour))

(event Game|Damage|EventAnyDamage
  (params (Damage :type Float%20%28single-precision%29) (DamageType :type Damage%20Type%20Object%20Reference) (InstigatedBy :type Controller%20Object%20Reference) (DamageCauser :type Actor%20Object%20Reference))
  ;[1 1 1] Start aiming player if damaged
  (if (> (Utilities|Array|FindItem (Variables|/Script/Engine.Actor|GetTags DamageCauser) (Utilities|Name|MakeLiteralName "Player")) -1)
    (CallFunction|StartAiming)
    (Variables|Default|SetIsAiming true)))

(event EventTick
  (params (DeltaSeconds :type Float%20%28single-precision%29))
  (Default|CallTickEvents DeltaSeconds)
  (Transformation|SetWorldRotation (Variables|Default|GetHealthBar) (Variables|Default|GetWidgetRotation) false false))

(event EventBeginPlay
  (bind _returnvalue (Game|GetPlayerController 0))
  (bind _returnvalue_2 (Pawn|GetControlledPawn _returnvalue))
  (bind _returnvalue_3 (Transformation|GetActorLocation _returnvalue_2))
  ;[1 1 1] Death
  (EventDispatchers|BindEventtoOnDeath (Variables|Default|GetTurretHealth) (delegate Custom|DeathEvent))
  ;[1 1 1] prepare shooting timer
  (bind _returnvalue_4 (Utilities|Time|SetTimerbyEvent (delegate Custom|ShootingEvent) (Variables|Default|GetShootingFrequency) true))
  (bind _output_get (Variables|Default|SetShootingTimer _returnvalue_4))
  (Utilities|Time|PauseTimerbyHandle _output_get)
  ;[1 1 1] Set Aim actor and ignor self
  (bind _outactors (Actor|GetAllActorsOfClasswithTag "/Game/MyContent/Blueprints/Character/BP_Character.BP_Character_C" "Player"))
  (Variables|Default|SetAimActor (Utilities|Array|Get(acopy) _outactors))
  (Utilities|Array|Add (Variables|Default|GetActors%20to%20Ignore) self)
  ;[1 1 1] Start behaviour
  (EventDispatchers|BindEventtoTickEvents (delegate Custom|BehaviourEvent))
  ;[1 1 1] Health bar rotation
  (Variables|Default|SetWidgetRotation (Math|Rotator|FindLookatRotation (+ (Transformation|GetActorForwardVector _returnvalue_2) _returnvalue_3) _returnvalue_3))
  ;[1 1 1] Bind health bar to health component
  (bind _asw_health_bar (Utilities|Casting|CastToW_HealthBar (UserInterface|GetWidget (Variables|Default|GetHealthBar))))
  (Class|GHealthComponent|SetWidget (Variables|Default|GetTurretHealth) _asw_health_bar)
  ;[1 1 1] Init From Save Data
  (CallFunction|CreateSaveDataProxy)
  (CallFunction|InitfromSave)
  (bind _asbp_start_game_mode (Utilities|Casting|CastToBP_StartGameMode (Game|GetGameMode)))
  (EventDispatchers|BindEventtoQuitGameEvent _asbp_start_game_mode (delegate Custom|SaveEvent)))

(fn ConstructionScript)

(fn IsAimed
  (params (AimLocation :type Vector) (Threshold :type Float%20%28single-precision%29))
  (return (< Threshold (/ (+ (Math|Vector|DotProduct (Math|Vector|Normalize (- AimLocation (Transformation|GetWorldLocation (Variables|Default|GetStaticMeshTop)))) (Math|Vector|GetForwardVector (Variables|Default|GetStaticMeshTop))) 1.0) 2.0))))

(fn HasLineOfSight
  (params (Object :type Actor%20Object%20Reference))
  (bind _outhit (Collision|LineTraceByChannel (Transformation|GetWorldLocation (Variables|Default|GetBarrelEndL)) (Transformation|GetActorLocation Object) "TraceTypeQuery1" false (Variables|Default|GetActors%20to%20Ignore) "None"))
  (return (== Object (.hitactor _outhit))))