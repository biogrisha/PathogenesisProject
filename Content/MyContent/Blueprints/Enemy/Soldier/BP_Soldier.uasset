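; Enemy soldier that carries a child-actor rifle and a health bar widget held at a rotation computed on BeginPlay.
; Shoot fires at a given target after a short delay; when shooting ends, the rifle reloads and a timer clears IsShooting.
; A save proxy registered with BP_StartGameMode restores location and health, and saves them on quit or on death before the actor is destroyed.
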(event Custom|DeathEvent
  (CallFunction|Save)
  (Actor|DestroyActor))

(event Custom|Shoot
  (params (Target :type Vector))
  (bind _rifle (Variables|Default|GetRifle))
  (bind _rifle_2 (Variables|Default|GetRifle))
  (Utilities|IsValid _rifle_2
    (:Is%20Valid
      (if (not (Variables|/Script/PathogenesisProject.GWeaponBase|GetbIsShooting _rifle_2))
        (Variables|Default|SetIsShooting true)
        (Utilities|FlowControl|Delay 0.4)
        (EventDispatchers|AssignShootingEnded _rifle (delegate Custom|ShootingEnded_Event_0))
        (Class|GWeaponBase|Shoot _rifle Target self)))))

(event Custom|Save
  (bind _output_get (Variables|Default|SetSaveData (Utilities|Struct|MakeDataToSave (Transformation|GetActorLocation) (Class|GHealthComponent|GetHealth (Variables|Default|GetSoldierHealth)) true)))
  (Class|GSaveDataProxy|SetData (Variables|Default|GetSaveDataProxy) _output_get))

(event Custom|ShootingEnded_Event_0
  (bind _rifle (Variables|Default|GetRifle))
  (EventDispatchers|UnbindallEventsfromShootingEnded (Variables|Default|GetRifle))
  (if (Utilities|Time|IsValidTimerHandle (Variables|Default|GetIsShootingTimer))
    (Utilities|Time|ClearandInvalidateTimerbyHandle (Variables|Default|GetIsShootingTimer)))
  (bind _returnvalue (Utilities|Time|SetTimerbyEvent (delegate Custom|UpdateIsShooting) 2.0))
  (Variables|Default|SetIsShootingTimer _returnvalue)
  (Class|GWeaponBase|Reload _rifle (Variables|/Script/PathogenesisProject.GWeaponBase|GetMagazineCapacity _rifle)))

(event Custom|CreateSaveDataProxy
  (bind _returnvalue (Game|GetGameMode))
  (bind _returnvalue_2 (Game|ConstructObjectfromClass "/Script/PathogenesisProject.GSaveDataProxy" _returnvalue))
  (bind _output_get (Variables|Default|SetSaveDataProxy _returnvalue_2))
  (Class|GSaveDataProxy|SetData _output_get (Utilities|Struct|MakeDataToSave (Transformation|GetActorLocation) (Class|GHealthComponent|GetHealth (Variables|Default|GetSoldierHealth)) false))
  (Class|GSaveDataProxy|SetStoredObjectName _output_get (Utilities|GetObjectName self))
  (bind _asbp_start_game_mode (Utilities|Casting|CastToBP_StartGameMode _returnvalue))
  (Default|SubscribeSaveDataProxy _asbp_start_game_mode _output_get)
  (bind _returnvalue_3 (Class|GSaveDataProxy|GetData _output_get))
  (Variables|Default|SetSaveData _returnvalue_3))

(event Custom|InitFromSave
  (bind _savedata (Variables|Default|GetSaveData))
  (Transformation|SetActorLocation (.location _savedata) false false)
  (Class|GHealthComponent|SetHealth (Variables|Default|GetSoldierHealth) (.health _savedata)))

(event Custom|SaveEvent
  ;[1 1 1] Init From Save Data
  (CallFunction|Save))

(event Custom|UpdateIsShooting
  (Variables|Default|SetIsShooting false))

(event EventBeginPlay
  (bind _returnvalue (Game|GetPlayerController 0))
  (bind _returnvalue_2 (Pawn|GetControlledPawn _returnvalue))
  (bind _returnvalue_3 (Transformation|GetActorLocation _returnvalue_2))
  (EventDispatchers|BindEventtoOnDeath (Variables|Default|GetSoldierHealth) (delegate Custom|DeathEvent))
  (bind _asw_health_bar (Utilities|Casting|CastToW_HealthBar (UserInterface|GetWidget (Variables|Default|GetWidget))))
  (Class|GHealthComponent|SetWidget (Variables|Default|GetSoldierHealth) _asw_health_bar)
  (Variables|Default|SetWidgetRotation (Math|Rotator|FindLookatRotation (+ (Transformation|GetActorForwardVector _returnvalue_2) _returnvalue_3) _returnvalue_3))
  ;[1 1 1] Init From Save Data
  (CallFunction|CreateSaveDataProxy)
  (CallFunction|InitfromSave)
  (bind _asbp_start_game_mode (Utilities|Casting|CastToBP_StartGameMode (Game|GetGameMode)))
  (EventDispatchers|BindEventtoQuitGameEvent _asbp_start_game_mode (delegate Custom|SaveEvent)))

(event EventTick
  (params (DeltaSeconds :type Float%20%28single-precision%29))
  (Transformation|SetWorldRotation (Variables|Default|GetWidget) (Variables|Default|GetWidgetRotation) false false))

(fn ConstructionScript
  (bind _asbp_rifle (Utilities|Casting|CastToBP_Rifle (Variables|/Script/Engine.ChildActorComponent|GetChildActor (Variables|Default|GetWeapon))))
  (bind _output_get (Variables|Default|SetRifle _asbp_rifle))
  (Variables|/Script/PathogenesisProject.GWeaponBase|SetDataAsset _output_get "/Game/MyContent/Blueprints/DataAssets/Weapon/DA_SuperRifle.DA_SuperRifle")
  (Collision|SetCollisionEnabled (Variables|/Game/MyContent/Blueprints/Weapons/BPWeapon.BPWeapon_C|GetCollision (Variables|Default|GetRifle)) "NoCollision"))