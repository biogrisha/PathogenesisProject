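; Weapon projectile Blueprint that damages what it hits, explodes and destroys itself, or expires two seconds after spawning.
; On sphere hit, it skips its Shooter and applies Damage only if the target or Shooter is tagged player, so non-player shooters cannot hurt each other.
; Damaging hits also report a damage event for AI perception.
; Every hit spawns a small explosion emitter, whether or not damage applies.
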(event OnComponentHit(Sphere)
  (params (HitComponent :type Primitive%20Component%20Object%20Reference) (OtherActor :type Actor%20Object%20Reference) (OtherComp :type Primitive%20Component%20Object%20Reference) (NormalImpulse :type Vector :default "0, 0, 0") (Hit :type Hit%20Result%20Structure%20%28by%20ref%29))
  (bind _damage (Variables|Default|GetDamage))
  (bind _shooter (Variables|Default|GetShooter))
  (if (and (Utilities|IsValid OtherActor) (Utilities|IsValid (Variables|Default|GetShooter)))
    (if (and (!= OtherActor (Variables|Default|GetShooter)) (or (Actor|ActorHasTag OtherActor "Player") (Actor|ActorHasTag (Variables|Default|GetShooter) "player")))
      (Game|Damage|ApplyDamage OtherActor _damage 0 _shooter)
      (Class|AISenseDamage|ReportDamageEvent OtherActor _shooter _damage (.location Hit) "0, 0, 0" "None")))
  (Effects|SpawnEmitteratLocation "/Game/StarterContent/Particles/P_Explosion.P_Explosion" (.location Hit) "0, 0, 0" "0.300000,0.300000,0.300000")
  (Actor|DestroyActor) ; Then destroy this projectile
)

(event EventBeginPlay
  (Utilities|FlowControl|Delay 2.0)
  (Actor|DestroyActor))

(fn ConstructionScript)