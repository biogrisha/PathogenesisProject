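; Weapon Blueprint that fires projectiles at a target, using a mesh and fire animation supplied by data assets.
; BeginPlay async-loads these assets, while item-data init applies them from an already loaded main weapon item and an unload event clears them.
; Shoot spends magazine ammo, plays the animation, spawns a projectile yawed toward the target with damage and shooter set, then signals shooting ended.
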(event Custom|SpawnProjectile
  (params (Target :type Vector) (Shooter :type Actor%20Object%20Reference))
  (bind _output_get (Variables|Default|SetNormalizedTarget (Math|Vector|Normalize (- Target (Transformation|GetActorLocation)))))
  (bind _returnvalue (Game|SpawnActorfromClass "/Game/MyContent/Blueprints/Weapons/Projectile.Projectile_C" (Math|Transform|MakeTransform (Transformation|GetWorldLocation (Variables|Default|GetProjectileSpawnPoint)) (Math|Rotator|MakeRotator 0.0 0.0 (.yaw (Math|Rotator|MakeRotfromXZ (Variables|Default|GetNormalizedTarget) (Math|Vector|CrossProduct (Math|Vector|CrossProduct _output_get "0, 0,1.000000") (Variables|Default|GetNormalizedTarget))))) "1,1,1") "AdjustIfPossibleButAlwaysSpawn" 0 0))
  (Variables|/Game/MyContent/Blueprints/Weapons/Projectile.Projectile_C|SetDamage _returnvalue (Variables|Default|GetWeaponDamage))
  (Variables|/Game/MyContent/Blueprints/Weapons/Projectile.Projectile_C|SetShooter _returnvalue Shooter))

(event EventBeginPlay
  (bind _dataasset (Variables|Default|GetDataAsset))
  (bind _output (Utilities|ResolveSoftReference _dataasset))
  (bind _mesh (Variables|/Script/PathogenesisProject.GGunDataAsset|GetMesh _output))
  ;[1 1 1] Load and set properties from Primary Data Asset
  (Utilities|AsyncLoadAsset _dataasset
    (:Completed
      (Utilities|IsValid (Utilities|ResolveSoftReference _dataasset)
        (:Is%20Valid
          (Utilities|AsyncLoadAsset (Variables|/Script/PathogenesisProject.GGunDataAsset|GetAnimation (Utilities|ResolveSoftReference _dataasset))
            (:Completed
              (Variables|Default|SetAnimation (Utilities|ResolveSoftReference (Variables|/Script/PathogenesisProject.GGunDataAsset|GetAnimation (Utilities|ResolveSoftReference _dataasset))))
              (Utilities|AsyncLoadAsset _mesh
                (:Completed
                  (Class|SkinnedMeshComponent|SetSkeletalMesh (Variables|Default|GetSkeletalMesh) (Utilities|ResolveSoftReference _mesh) true))))))))))

(event EventInitfromItemDataBP
  (params (Data :type G%20Inventory%20Item%20Base%20Object%20Reference))
  (Utilities|IsValid Data
    (:Is%20Valid
      (bind _asginventory_item_main_weapon (Utilities|Casting|CastToGInventoryItemMainWeapon Data))
      (if (Class|GInventoryItemBase|IsAssetLoaded _asginventory_item_main_weapon)
        (bind _asggun_data_asset (Utilities|Casting|CastToGGunDataAsset (Class|GInventoryItemBase|GetDataAsset _asginventory_item_main_weapon)))
        (Variables|Default|SetAnimation (Utilities|ResolveSoftReference (Variables|/Script/PathogenesisProject.GGunDataAsset|GetAnimation _asggun_data_asset)))
        (Class|SkinnedMeshComponent|SetSkeletalMesh (Variables|Default|GetSkeletalMesh) (Utilities|ResolveSoftReference (Variables|/Script/PathogenesisProject.GGunDataAsset|GetMesh _asggun_data_asset)) true)))))

(event EventUnloadAssetsBP
  (Class|SkinnedMeshComponent|SetSkeletalMesh (Variables|Default|GetSkeletalMesh) 0 true)
  (Variables|Default|SetAnimation 0))

(event EventShoot
  (params (Target :type Vector%20%28by%20ref%29 :default "0, 0, 0") (Shooter :type Actor%20Object%20Reference))
  (bind _currentmagazine (Variables|Default|GetCurrentMagazine))
  (Variables|Default|SetTarget Target)
  (if (> _currentmagazine 0)
    (Class|GWeaponBase|SetCurrentMagazine (- _currentmagazine 1))
    (Components|Animation|PlayAnimation (Variables|Default|GetSkeletalMesh) (Variables|Default|GetAnimation) false)
    (CallFunction|SpawnProjectile (Variables|Default|GetTarget) Shooter)
    (Default|CallShootingEnded)))

(fn ConstructionScript)