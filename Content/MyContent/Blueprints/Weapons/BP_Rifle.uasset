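; BP_Rifle is a rifle weapon Blueprint that fires short automatic bursts at a given target.
; Shoot ignores calls while already shooting, then loops through a Gate and Delay to play the fire animation, spend magazine ammo and spawn a projectile.
; When the burst limit is reached or the magazine empties, it resets its state, signals that shooting ended and closes the gate.
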(event EventBeginPlay)

(event Collision|EventActorBeginOverlap
  (params (OtherActor :type Actor%20Object%20Reference)))

(event EventTick
  (params (DeltaSeconds :type Float%20%28single-precision%29)))

(event EventShoot
  (params (Target :type Vector%20%28by%20ref%29 :default "0, 0, 0") (Shooter :type Actor%20Object%20Reference))
  (bind _currentmagazine (Variables|Default|GetCurrentMagazine))
  (if (not (Variables|Default|GetbIsShooting))
    (Variables|Default|SetTarget_0 Target)
    (Variables|Default|SetbIsShooting true)
    (Utilities|FlowControl|Sequence
      (:then_0
        (goto _label Open))
      (:then_1
        (Utilities|FlowControl|Gate false :!label _label
          (:Exit
            (if (and (< (Variables|Default|GetShootingCounter) 4) (> _currentmagazine 0))
              (Math|Integer|IncrementInt (Variables|Default|GetShootingCounter)
                (:%20%20
                  (Class|GWeaponBase|SetCurrentMagazine (- _currentmagazine 1))
                  (Components|Animation|PlayAnimation (Variables|Default|GetSkeletalMesh) (Variables|Default|GetAnimation) false)
                  (CallFunction|SpawnProjectile (Variables|Default|GetTarget_0) Shooter)
                  (Utilities|FlowControl|Delay 0.1)
                  (goto _label)))
              (else
                (Variables|Default|SetbIsShooting false)
                (Variables|Default|SetShootingCounter 0)
                (Default|CallShootingEnded)
                (goto _label Close)))))))))

(fn ConstructionScript
  (|CallParentFunction))