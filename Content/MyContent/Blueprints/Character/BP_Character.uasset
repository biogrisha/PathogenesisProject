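; Player-controlled character that walks toward an ordered location and turns in yaw to follow the mouse cursor.
; Tick feeds movement input toward the target and derives facing by projecting the cursor offset onto the view plane.
; Active and concealed weapons attach to hand and spine sockets and swap with weapon mode; IsShooting clears on a delay after firing ends.
; The controlling Player receives overlapped pickables and forwarded damage.
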(event OnComponentBeginOverlap(CapsuleComponent)
  (params (OverlappedComponent :type Primitive%20Component%20Object%20Reference) (OtherActor :type Actor%20Object%20Reference) (OtherComp :type Primitive%20Component%20Object%20Reference) (OtherBodyIndex :type Integer) (bFromSweep :type Boolean) (SweepResult :type Hit%20Result%20Structure%20%28by%20ref%29))
  (bind _asgpickable_base (Utilities|Casting|CastToGPickableBase OtherActor))
  (Default|SetFindedItem (Variables|Default|GetPlayer) _asgpickable_base))

(event Custom|DirectToLocation
  (params (GoToLocation :type Vector))
  (Variables|Default|SetGoToPos GoToLocation))

(event Custom|Shoot
  (params (Target :type Vector))
  (bind _activeweapon (Variables|Default|GetActiveWeapon))
  (bind _activeweapon_2 (Variables|Default|GetActiveWeapon))
  (Utilities|IsValid _activeweapon_2
    (:Is%20Valid
      (if (not (Variables|/Script/PathogenesisProject.GWeaponBase|GetbIsShooting _activeweapon_2))
        (Variables|Default|SetIsShooting true)
        (Utilities|FlowControl|Delay 0.2)
        (EventDispatchers|AssignShootingEnded _activeweapon (delegate Custom|ShootingEnded_Event_0))
        (Class|GWeaponBase|Shoot _activeweapon Target self)))))

(event Custom|EquipActiveWeapon
  (params (Weapon :type BP%20Weapon%20Object%20Reference))
  (bind _output_get (Variables|Default|SetActiveWeapon Weapon))
  (Utilities|IsValid _output_get
    (:Is%20Valid
      (Transformation|DetachFromActor Weapon "KeepWorld" "KeepWorld" "KeepWorld")
      (Collision|SetCollisionEnabled (Variables|/Game/MyContent/Blueprints/Weapons/BPWeapon.BPWeapon_C|GetCollision Weapon) "NoCollision")
      (Transformation|SetActorTransform Weapon)
      (Transformation|AttachComponentToComponent Weapon (Variables|Character|GetMesh) "Arm_RSocket" "KeepRelative" "KeepRelative" "KeepRelative" true))))

(event Custom|EquipConcealedWeapon
  (params (Weapon :type BP%20Weapon%20Object%20Reference))
  (bind _output_get (Variables|Default|SetConcealedWeapon Weapon))
  (Utilities|IsValid _output_get
    (:Is%20Valid
      (Transformation|DetachFromActor Weapon "KeepWorld" "KeepWorld" "KeepWorld")
      (Collision|SetCollisionEnabled (Variables|/Game/MyContent/Blueprints/Weapons/BPWeapon.BPWeapon_C|GetCollision Weapon) "NoCollision")
      (Transformation|SetActorTransform Weapon)
      (Transformation|AttachComponentToComponent Weapon (Variables|Character|GetMesh) "Spine1Socket" "KeepRelative" "KeepRelative" "KeepRelative" true))))

(event Custom|SetActiveWeaponMode
  (params (Mode :type E_ActiveItem%20Enum :default "NewEnumerator0"))
  (if (not (Utilities|Enum|Equal(Enum) Mode (Variables|Default|GetWeaponMode)))
    (Variables|Default|SetWeaponMode Mode)
    (Variables|Default|SetActiveWeaponTemp (Variables|Default|GetActiveWeapon))
    (CallFunction|EquipActiveWeapon (Variables|Default|GetConcealedWeapon))
    (CallFunction|EquipConcealedWeapon (Variables|Default|GetActiveWeaponTemp))))

(event Custom|EquipWeapon
  (params (NewParam :type BP%20Weapon%20Object%20Reference))
  (bind _itemtype (Variables|/Script/PathogenesisProject.GPickableBase|GetItemType NewParam))
  (switch Utilities|FlowControl|Switch|SwitchonE_ActiveItem (Variables|Default|GetWeaponMode)
    (:NewEnumerator0
      (switch Utilities|FlowControl|Switch|SwitchonEItemType _itemtype
        (:MainWeapon
          (CallFunction|EquipActiveWeapon NewParam))
        (:SecondaryWeapon
          (CallFunction|EquipConcealedWeapon NewParam))))
    (:NewEnumerator1
      (switch Utilities|FlowControl|Switch|SwitchonEItemType _itemtype
        (:MainWeapon
          (CallFunction|EquipConcealedWeapon NewParam))
        (:SecondaryWeapon
          (CallFunction|EquipActiveWeapon NewParam))))))

(event Custom|ShootingEnded_Event_0
  (EventDispatchers|UnbindallEventsfromShootingEnded (Variables|Default|GetActiveWeapon))
  (if (Utilities|Time|IsValidTimerHandle (Variables|Default|GetUpdateIsShootingTimer))
    (Utilities|Time|ClearandInvalidateTimerbyHandle (Variables|Default|GetUpdateIsShootingTimer)))
  (bind _returnvalue (Utilities|Time|SetTimerbyEvent (delegate Custom|UpdateIsShooting) 2.0))
  (Variables|Default|SetUpdateIsShootingTimer _returnvalue))

(event Custom|UpdateIsShooting
  (Variables|Default|SetIsShooting false))

(event EventBeginPlay
  (Variables|Default|SetGoToPos (Transformation|GetActorLocation)))

(event Game|Damage|EventAnyDamage
  (params (Damage :type Float%20%28single-precision%29) (DamageType :type Damage%20Type%20Object%20Reference) (InstigatedBy :type Controller%20Object%20Reference) (DamageCauser :type Actor%20Object%20Reference))
  (Game|Damage|ApplyDamage (Variables|Default|GetPlayer) Damage 0 DamageCauser))

(event EventTick
  (params (DeltaSeconds :type Float%20%28single-precision%29))
  (CallFunction|CalcRotation)
  ;[1 1 1] Lead фт actor to click position
  (bind _output_get (Variables|Default|SetDirection (- (Variables|Default|GetGoToPos) (Transformation|GetActorLocation))))
  (if (> (Math|Vector|VectorLengthSquared _output_get) 2.5e+03)
    (Class|PawnMovementComponent|AddInputVector (Variables|Character|GetCharacterMovement) (* (Math|Vector|Normalize (Variables|Default|GetDirection) 0.3) 0.5) false)))

(event EventSetControllingPlayer
  (params (ControllingPlayer :type BP%20Player%20Object%20Reference))
  (Variables|Default|SetPlayer ControllingPlayer))

(fn ConstructionScript)

(fn CalcRotation
  (bind _returnvalue (Game|GetPlayerController 0))
  (bind _returnvalue_2 (Transformation|GetActorLocation))
  (bind _returnvalue_3 (Transformation|GetActorForwardVector _returnvalue))
  (bind _output_get (LocalVariables|SetMouseLocation (.WorldLocation (Game|Player|ConvertMouseLocationToWorldSpace _returnvalue))))
  (bind _output_get_2 (LocalVariables|SetActorLocOrigin (- (Transformation|GetActorLocation) _output_get)))
  (Transformation|SetActorRotation (Math|Rotator|MakeRotator 0.0 0.0 (.yaw (Math|Rotator|FindLookatRotation _returnvalue_2 (- _returnvalue_2 (Math|Vector|MakeVector (.x (- _output_get_2 (* _returnvalue_3 (Math|Vector|DotProduct _output_get_2 _returnvalue_3)))) (.y (- _output_get_2 (* _returnvalue_3 (Math|Vector|DotProduct _output_get_2 _returnvalue_3)))) (.z (Transformation|GetActorLocation)))))))))