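; Game mode that shows the mouse cursor and manages the game's single save slot, including new game and quit handling.
; Data proxies register through SubscribeSaveDataProxy, which lazily loads or creates the GMySaveGame and restores each proxy's data by stored object name.
; SaveGame copies all registered proxy data back into that object and writes it asynchronously.
; Quitting fires a quit event and saves first, while NewGame deletes the slot and restarts.
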(event Custom|SaveGame
  (CallFunction|LoadProxiestoSaveData)
  (|AsyncSaveGametoSlot (Variables|Default|GetSaveData) "save1"))

(event Custom|CustomQuitGame
  (Default|CallQuitGameEvent)
  (CallFunction|SaveGame)
  (Game|QuitGame 0 "Quit" false))

(event Custom|LoadProxiesToSaveData
  (for _array_element (Variables|Default|GetSaveDataProxies)
    (bind _returnvalue (Class|GSaveDataProxy|GetStoredObjectName _array_element))
    (bind _returnvalue_2 (Class|GSaveDataProxy|GetData _array_element))
    (Class|GMySaveGame|UpdateData (Variables|Default|GetSaveData) _returnvalue_2 _returnvalue)))

(event Custom|NewGame
  (SaveGame|DeleteGameinSlot "save1")
  (Class|GameMode|RestartGame))

(event EventBeginPlay
  (Variables|/Script/Engine.PlayerController|SetbShowMouseCursor (Game|GetPlayerController 0) true))

(event EventTick
  (params (DeltaSeconds :type Float%20%28single-precision%29)))

(fn ConstructionScript)

(fn SubscribeSaveDataProxy
  (params (DataProxy :type G%20Save%20Data%20Proxy%20Object%20Reference))
  (Utilities|IsValid (Variables|Default|GetSaveData)
    (:Is%20Valid
      _)
    (:Is%20Not%20Valid
      (bind _returnvalue (SaveGame|DoesSaveGameExist "save1"))
      (if _returnvalue
        (bind _returnvalue_2 (SaveGame|LoadGamefromSlot "save1"))
        (bind _asgmy_save_game (Utilities|Casting|CastToGMySaveGame _returnvalue_2))
        (Variables|Default|SetSaveData _asgmy_save_game)
        (else
          ;[1 1 1] Create Save File
          (bind _returnvalue_3 (SaveGame|CreateSaveGameObject "/Script/PathogenesisProject.GMySaveGame"))
          (Variables|Default|SetSaveData _returnvalue_3)
          (SaveGame|SaveGametoSlot _returnvalue_3 "save1")))))
  (bind _returnvalue_4 (Class|GSaveDataProxy|GetStoredObjectName DataProxy))
  (bind (_outdata _returnvalue_5) (Class|GMySaveGame|LoadData (Variables|Default|GetSaveData) _returnvalue_4))
  (if _returnvalue_5
    (Class|GSaveDataProxy|SetData DataProxy _outdata))
  (Utilities|Array|Add (Variables|Default|GetSaveDataProxies) DataProxy))